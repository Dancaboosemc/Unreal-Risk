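; Turn manager for a Risk game that loads player names, colors and difficulties from the game instance.
; AiCheck branches on phase: begin and reinforcement reset board events, then enable the user's input or spawn AI handler actors.
; User reinforcement also sets troop counts and refreshes the in-game menu.
; AI difficulty selects the begin and attack handlers; reinforcement always uses the easy one, and attack skips the user check.
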(event Custom|Event%20AiCheck
  (bind _returnvalue (Math|Transform|MakeTransform "0, 0, 0"))
  (bind _returnvalue_2 (Math|Transform|MakeTransform "0, 0, 0"))
  (bind _returnvalue_3 (Class|TurnHandler|GetCurrentPhase))
  (switch Utilities|FlowControl|Switch|SwitchonEPhases _returnvalue_3
    (:BEGIN
      (bind _outactors (Actor|GetAllActorsOfClass "/Script/UnrealRisk.Board"))
      (for _array_element _outactors
        (Class|Board|TurnOffBoardEvents _array_element))
      (bind _returnvalue_4 (Class|TurnHandler|GetCurrentPlayer))
      (if (Utilities|Enum|Equal(Enum) _returnvalue_4 "USER")
        (bind _outactors_2 (Actor|GetAllActorsOfClass "/Script/UnrealRisk.Board"))
        (for _array_element_2 _outactors_2
          (Class|Board|TurnonUnclaimedEvents _array_element_2))
        (else
          (bind _returnvalue_5 (Class|TurnHandler|GetDifficulty (Math|Conversions|ToInteger(Byte) _returnvalue_4)))
          (if (Utilities|Enum|Equal(Enum) _returnvalue_5 "EASY")
            (Game|SpawnActorfromClass "/Game/RiskContent/BluePrints/EasyBeginAiHandler.EasyBeginAiHandler_C" _returnvalue_2 "Undefined" 0 0)
            (else
              (Game|SpawnActorfromClass "/Game/RiskContent/BluePrints/HardBeginAiHandler.HardBeginAiHandler_C" _returnvalue_2 "Undefined" 0 0))))))
    (:REINF
      (bind _outactors_3 (Actor|GetAllActorsOfClass "/Script/UnrealRisk.Board"))
      (for _array_element_3 _outactors_3
        (Class|Board|TurnOffBoardEvents _array_element_3))
      (bind _returnvalue_6 (Class|TurnHandler|GetCurrentPlayer))
      (if (Utilities|Enum|Equal(Enum) _returnvalue_6 "USER")
        (bind _outactors_4 (Actor|GetAllActorsOfClass "/Script/UnrealRisk.Board"))
        (for _array_element_4 _outactors_4
          (Class|Board|TurnonPlayerSpaceEvents _array_element_4)
          (bind _returnvalue_7 (Class|TurnHandler|GetReinforcments (Math|Conversions|ToInteger(Byte) _returnvalue_6)))
          (Class|TurnHandler|SetCurrentReinfTroops _returnvalue_7)
          (bind _foundwidgets (Widget|GetAllWidgetsOfClass "/Game/RiskContent/UMG/InGameMenuWidget.InGameMenuWidget_C" true))
          (for _array_element_5 _foundwidgets
            (Default|ReinforcmentUpdate _array_element_5)))
        (else
          (Game|SpawnActorfromClass "/Game/RiskContent/BluePrints/EasyReinfAiHandler.EasyReinfAiHandler_C" (Math|Transform|MakeTransform "0, 0, 0") "Undefined" 0 0))))
    (:ATTACK
      (bind _returnvalue_8 (Class|TurnHandler|GetCurrentPlayer))
      (bind _returnvalue_9 (Class|TurnHandler|GetDifficulty (Math|Conversions|ToInteger(Byte) _returnvalue_8)))
      (switch Utilities|FlowControl|Switch|SwitchonEDifficulties _returnvalue_9
        (:EASY
          (Game|SpawnActorfromClass "/Game/RiskContent/BluePrints/EasyAIAttackHandler.EasyAIAttackHandler_C" _returnvalue "Undefined" 0 0))
        (:HARD
          (Game|SpawnActorfromClass "/Game/RiskContent/BluePrints/HardAIAttackHandler.HardAIAttackHandler_C" _returnvalue "Undefined" 0 0))))))

(event EventBeginPlay
  (bind _asunreal_risk_game_instance (Utilities|Casting|CastToUnrealRiskGameInstance (Game|GetGameInstance)))
  (Class|TurnHandler|SetMembers (Variables|/Game/RiskContent/BluePrints/UnrealRiskGameInstance.UnrealRiskGameInstance_C|GetPlayerNames _asunreal_risk_game_instance) (Variables|/Game/RiskContent/BluePrints/UnrealRiskGameInstance.UnrealRiskGameInstance_C|GetPlayerColors _asunreal_risk_game_instance) (Variables|/Game/RiskContent/BluePrints/UnrealRiskGameInstance.UnrealRiskGameInstance_C|GetPlayerDifficulties _asunreal_risk_game_instance)))

(event Collision|EventActorBeginOverlap
  (params (OtherActor :type Actor%20Object%20Reference)))

(event EventTick
  (params (DeltaSeconds :type Float%20%28single-precision%29)))

(fn ConstructionScript)