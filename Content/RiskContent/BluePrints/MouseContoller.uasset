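; Input controller that pans and zooms the "Main"-tagged CameraActor within fixed bounds.
; W, A, S and D pan on X and Y by re-triggering a local Hold macro, built from a retriggerable delay and gates, until key release or a limit.
; The mouse wheel steps height, and zooming out also eases X and Y proportionally toward the origin, so the camera is centered at maximum height.
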(event EventBeginPlay)

(event EventTick
  (params (DeltaSeconds :type Float%20%28single-precision%29)))

(event Input|MouseEvents|MouseWheelDown
  (params (Key :type Key%20Structure :default "None"))
  (:Pressed
    (bind _outactors (Actor|GetAllActorsOfClasswithTag "/Script/Engine.CameraActor" "Main"))
    (for _array_element _outactors
      (if (not (>= (.z (.location (Transformation|GetActorTransform _array_element))) 2.6e+02))
        (Transformation|SetActorTransform _array_element (Math|Transform|MakeTransform (Math|Vector|MakeVector (+ (.x (.location (Transformation|GetActorTransform _array_element))) (/ (- 0.0 (.x (.location (Transformation|GetActorTransform _array_element)))) (/ (- 2.6e+02 (.z (.location (Transformation|GetActorTransform _array_element)))) 2e+01))) (+ (.y (.location (Transformation|GetActorTransform _array_element))) (/ (- 0.0 (.y (.location (Transformation|GetActorTransform _array_element)))) (/ (- 2.6e+02 (.z (.location (Transformation|GetActorTransform _array_element)))) 2e+01))) (+ (.z (.location (Transformation|GetActorTransform _array_element))) 2e+01)) (.rotation (Transformation|GetActorTransform _array_element)) (.scale (Transformation|GetActorTransform _array_element))))))))

(event Input|MouseEvents|MouseWheelUp
  (params (Key :type Key%20Structure :default "None"))
  (:Pressed
    (bind _outactors (Actor|GetAllActorsOfClasswithTag "/Script/Engine.CameraActor" "Main"))
    (for _array_element _outactors
      (if (not (<= (.z (.location (Transformation|GetActorTransform _array_element))) 1e+02))
        (Transformation|SetActorTransform _array_element (Math|Transform|MakeTransform (Math|Vector|MakeVector (.x (.location (Transformation|GetActorTransform _array_element))) (.y (.location (Transformation|GetActorTransform _array_element))) (- (.z (.location (Transformation|GetActorTransform _array_element))) 2e+01)) (.rotation (Transformation|GetActorTransform _array_element)) (.scale (Transformation|GetActorTransform _array_element))))))))

(event Input|KeyboardEvents|W
  (params (Key :type Key%20Structure :default "None"))
  (:Pressed
    (Utilities|Hold 0.005 :!label _label
      (:Hold
        (bind _outactors (Actor|GetAllActorsOfClasswithTag "/Script/Engine.CameraActor" "Main"))
        (for _array_element _outactors
          (if (not (<= (.y (.location (Transformation|GetActorTransform _array_element))) -1e+02))
            (Transformation|SetActorTransform _array_element (Math|Transform|MakeTransform (Math|Vector|MakeVector (.x (.location (Transformation|GetActorTransform _array_element))) (- (.y (.location (Transformation|GetActorTransform _array_element))) 2.0) (.z (.location (Transformation|GetActorTransform _array_element)))) (.rotation (Transformation|GetActorTransform _array_element)) (.scale (Transformation|GetActorTransform _array_element))))
            (goto _label))))))
  (:Released
    (goto _label Released)))

(event Input|KeyboardEvents|D
  (params (Key :type Key%20Structure :default "None"))
  (:Pressed
    (Utilities|Hold 0.005 :!label _label
      (:Hold
        (bind _outactors (Actor|GetAllActorsOfClasswithTag "/Script/Engine.CameraActor" "Main"))
        (for _array_element _outactors
          (if (not (>= (.x (.location (Transformation|GetActorTransform _array_element))) 125.0))
            (Transformation|SetActorTransform _array_element (Math|Transform|MakeTransform (Math|Vector|MakeVector (+ (.x (.location (Transformation|GetActorTransform _array_element))) 2.0) (.y (.location (Transformation|GetActorTransform _array_element))) (.z (.location (Transformation|GetActorTransform _array_element)))) (.rotation (Transformation|GetActorTransform _array_element)) (.scale (Transformation|GetActorTransform _array_element))))
            (goto _label))))))
  (:Released
    (goto _label Released)))

(event Input|KeyboardEvents|S
  (params (Key :type Key%20Structure :default "None"))
  (:Pressed
    (Utilities|Hold 0.005 :!label _label
      (:Hold
        (bind _outactors (Actor|GetAllActorsOfClasswithTag "/Script/Engine.CameraActor" "Main"))
        (for _array_element _outactors
          (if (not (>= (.y (.location (Transformation|GetActorTransform _array_element))) 1e+02))
            (Transformation|SetActorTransform _array_element (Math|Transform|MakeTransform (Math|Vector|MakeVector (.x (.location (Transformation|GetActorTransform _array_element))) (+ (.y (.location (Transformation|GetActorTransform _array_element))) 2.0) (.z (.location (Transformation|GetActorTransform _array_element)))) (.rotation (Transformation|GetActorTransform _array_element)) (.scale (Transformation|GetActorTransform _array_element))))
            (goto _label))))))
  (:Released
    (goto _label Released)))

(event Input|KeyboardEvents|A
  (params (Key :type Key%20Structure :default "None"))
  (:Pressed
    (Utilities|Hold 0.005 :!label _label
      (:Hold
        (bind _outactors (Actor|GetAllActorsOfClasswithTag "/Script/Engine.CameraActor" "Main"))
        (for _array_element _outactors
          (if (not (<= (.x (.location (Transformation|GetActorTransform _array_element))) -125.0))
            (Transformation|SetActorTransform _array_element (Math|Transform|MakeTransform (Math|Vector|MakeVector (- (.x (.location (Transformation|GetActorTransform _array_element))) 2.0) (.y (.location (Transformation|GetActorTransform _array_element))) (.z (.location (Transformation|GetActorTransform _array_element)))) (.rotation (Transformation|GetActorTransform _array_element)) (.scale (Transformation|GetActorTransform _array_element))))
            (goto _label))))))
  (:Released
    (goto _label Released)))

(fn ConstructionScript)